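; Player sound component that appears to be an unfinished footstep audio prototype.
; BeginPlay spawns an attached audio component and stores it, while the shoot and dash inputs only print debug text.
; PlayFootsteps plays that component when a capsule-sized sphere trace from the BP_SuperCharacter owner hits, but sets no specific sound.
; Its call and the velocity-driven footstep timeline are disconnected, so footsteps never trigger from this graph.
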(event Input|EnhancedActionEvents|EnhancedInputActionIA_Shoot
  (params (ActionValue :type Boolean) (ElapsedSeconds :type Float%20%28double-precision%29) (TriggeredSeconds :type Float%20%28double-precision%29) (InputAction :type Input%20Action%20Object%20Reference :default "/Game/Blueprints/PlayerController/IA_Shoot.IA_Shoot"))
  (Development|PrintString "SHOOOOOT"))

(event Input|EnhancedActionEvents|EnhancedInputActionIA_Dash
  (params (ActionValue :type Boolean) (ElapsedSeconds :type Float%20%28double-precision%29) (TriggeredSeconds :type Float%20%28double-precision%29) (InputAction :type Input%20Action%20Object%20Reference :default "/Game/Blueprints/PlayerController/IA_Dash.IA_Dash"))
  (Development|PrintString "DASH!"))

(event EventBeginPlay
  (bind _returnvalue (Audio|SpawnSoundAttached 0 (Class|Actor|GetParentComponent (Components|GetOwner)) "None" "0, 0, 0" "0, 0, 0" "KeepRelativeOffset" false 1.0 1.0 0.0 0 0))
  (Variables|Default|SetPlayerAudioComponent _returnvalue))

(event EventTick
  (params (DeltaSeconds :type Float%20%28single-precision%29)))

(fn PlayFootsteps
  (bind _playeraudiocomponent (Variables|Default|GetPlayerAudioComponent))
  (bind _finished (CallFunction|TraceFootSteps))
  (if _finished
    (Audio|Components|Audio|SetSound _playeraudiocomponent 0)
    (Audio|Components|Audio|Play _playeraudiocomponent 0.0)))

(fn TraceFootSteps
  (bind _returnvalue (Components|GetOwner))
  (bind _asbp_super_character (Utilities|Casting|CastToBP_SuperCharacter _returnvalue))
  (bind _returnvalue_2 (Collision|SphereTraceByChannel (Transformation|GetActorLocation _returnvalue) (Math|Vector|MakeVector 0.0 0.0 (- 0.0 (Components|Capsule|GetScaledCapsuleHalfHeight (Variables|/Script/Engine.Character|GetCapsuleComponent _asbp_super_character)))) (Components|Capsule|GetScaledCapsuleRadius (Variables|/Script/Engine.Character|GetCapsuleComponent _asbp_super_character)) "TraceTypeQuery1" false 0 "None"))
  (return _returnvalue_2))