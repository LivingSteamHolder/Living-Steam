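; Player sound actor, parented to the character, that plays audio for footsteps, jumps, landings, dashes, shooting and death.
; Input events and per-tick checks of BP_SuperCharacter state fire trigger parameters on footstep, dash and shooting audio components, with DoOnce gates limiting repeats.
; A timeline paces footsteps while walking, using a downward sphere trace before triggering a rock step.
; Charge-shot audio fades out on cancel; death plays a randomized 2D voice.
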(event Input|EnhancedActionEvents|EnhancedInputActionIA_Dash
  (params (ActionValue :type Boolean) (ElapsedSeconds :type Float%20%28double-precision%29) (TriggeredSeconds :type Float%20%28double-precision%29) (InputAction :type Input%20Action%20Object%20Reference :default "/Game/Blueprints/PlayerController/IA_Dash.IA_Dash"))
  (Utilities|FlowControl|DoOnce false
    (:Completed
      (Class|AudioParameterControllerInterface|SetTriggerParameter (Variables|Default|GetMSS_Dash) "Dash"))))

(event Input|EnhancedActionEvents|EnhancedInputActionIA_Shoot
  (params (ActionValue :type Boolean) (ElapsedSeconds :type Float%20%28double-precision%29) (TriggeredSeconds :type Float%20%28double-precision%29) (InputAction :type Input%20Action%20Object%20Reference :default "/Game/Blueprints/PlayerController/IA_Shoot.IA_Shoot"))
  (:Triggered
    (Variables|Default|SetStopShootingLoop true)
    (Class|AudioParameterControllerInterface|SetTriggerParameter (Variables|Default|GetMSS_Shooting) "Shot"))
  (:Started
    (Audio|Components|Audio|FadeIn (Variables|Default|GetMSS_Shooting) 0.0 1.0 0.0 "Linear" :!class /Script/Engine.AudioComponent)))

(event Input|EnhancedActionEvents|EnhancedInputActionIA_Jump
  (params (ActionValue :type Boolean) (ElapsedSeconds :type Float%20%28double-precision%29) (TriggeredSeconds :type Float%20%28double-precision%29) (InputAction :type Input%20Action%20Object%20Reference :default "/Game/Blueprints/PlayerController/IA_Jump.IA_Jump"))
  (:Started
    (Utilities|FlowControl|DoOnce false
      (:Completed
        (Class|AudioParameterControllerInterface|SetTriggerParameter (Variables|Default|GetMSS_Footstep) "Jump")
        (Components|Timeline|SetPlaybackPosition (Variables|Default|GetTL_Footsteps) 0.0 false true)
        (Utilities|FlowControl|DoOnce true) ; enters at Reset
      ))))

(event Input|EnhancedActionEvents|EnhancedInputActionIA_ChargeShoot
  (params (ActionValue :type Boolean) (ElapsedSeconds :type Float%20%28double-precision%29) (TriggeredSeconds :type Float%20%28double-precision%29) (InputAction :type Input%20Action%20Object%20Reference :default "/Game/Blueprints/PlayerController/IA_ChargeShoot.IA_ChargeShoot"))
  (:Triggered
    (Variables|Default|SetStopShootingLoop true)
    (Class|AudioParameterControllerInterface|SetTriggerParameter (Variables|Default|GetMSS_Shooting) "Shot"))
  (:Started
    (Audio|Components|Audio|FadeIn (Variables|Default|GetMSS_Shooting) 0.0 1.0 0.0 "Linear" :!class /Script/Engine.AudioComponent)
    (Class|AudioParameterControllerInterface|SetTriggerParameter (Variables|Default|GetMSS_Shooting) "Shoot")
    (Variables|Default|SetStopShootingLoop false))
  (:Canceled
    (Development|PrintString "CANCELED")
    (Audio|Components|Audio|FadeOut (Variables|Default|GetMSS_Shooting) 1.0 0.0 "Linear" :!class /Script/Engine.AudioComponent)
    (Class|AudioParameterControllerInterface|SetTriggerParameter (Variables|Default|GetMSS_Shooting) "Canceled")
    (Development|PrintString "CANCEL!")))

(event EventBeginPlay
  (bind _asbp_super_character (Utilities|Casting|CastToBP_SuperCharacter (Game|GetPlayerCharacter 0)))
  (Variables|Default|SetCharacterMovement (Variables|/Script/Engine.Character|GetCharacterMovement _asbp_super_character))
  (Variables|Default|SetPlayerBP _asbp_super_character)
  (Variables|Default|SetStopShootingLoop true))

(event EventTick
  (params (DeltaSeconds :type Float%20%28single-precision%29))
  (bind _returnvalue (Math|Random|RandomFloatinRange 0.7 0.9))
  (bind _tl_footsteps (Variables|Default|GetTL_Footsteps))
  (Utilities|FlowControl|Sequence
    (:then_0
      (if (and (> (Math|Vector|VectorLength (Transformation|GetVelocity (Actor|GetParentActor))) 0.0) (Pawn|Components|CharacterMovement|IsWalking (Variables|Default|GetCharacterMovement)))
        (Components|Timeline|SetPlayRate _tl_footsteps (Variables|Default|GetFootPlayRate))
        (Audio|Components|Audio|Play _tl_footsteps)
        (else
          (Audio|Components|Audio|Stop _tl_footsteps))))
    (:then_1
      (if (<= (Variables|/Script/LivingSteam.SuperCharacterClass|GetDashCurrentCooldown (Variables|Default|GetPlayerBP)) 0.04)
        (Utilities|FlowControl|DoOnce false) ; enters at Reset
      ))
    (:then_2
      (if (Pawn|Components|CharacterMovement|IsWalking (Variables|Default|GetCharacterMovement))
        (Utilities|FlowControl|DoOnce true
          (:Completed
            (Class|AudioParameterControllerInterface|SetTriggerParameter (Variables|Default|GetMSS_Footstep) "Land")))))
    (:then_3
      (if (Pawn|Components|CharacterMovement|IsWalking (Variables|Default|GetCharacterMovement))
        (Utilities|FlowControl|DoOnce false) ; enters at Reset
      ))
    (:then_5
      (if (Variables|Default|GetStopShootingLoop)
        (Class|AudioParameterControllerInterface|SetTriggerParameter (Variables|Default|GetMSS_Shooting) "Stop")))
    (:then_6
      (if (Variables|/Script/LivingSteam.SuperCharacterClass|GetIsDead (Variables|Default|GetPlayerBP))
        (Utilities|FlowControl|DoOnce false
          (:Completed
            (Audio|PlaySound2D "/Game/Sounds/Waves/Voice/SW_Voice1.SW_Voice1" _returnvalue _returnvalue 0.0 0 0)))))))

(fn ConstructionScript)

(fn PlayFootsteps
  (bind _finished (CallFunction|TraceFootSteps))
  (if _finished
    (Class|AudioParameterControllerInterface|SetTriggerParameter (Variables|Default|GetMSS_Footstep) "RockStep")))

(fn TraceFootSteps
  (bind _asbp_super_character (Utilities|Casting|CastToBP_SuperCharacter (Actor|GetParentActor)))
  (bind _returnvalue (Collision|SphereTraceByChannel (Transformation|GetActorLocation (Actor|GetParentActor)) (Math|Vector|MakeVector 0.0 0.0 (- 0.0 (Components|Capsule|GetScaledCapsuleHalfHeight (Variables|/Script/Engine.Character|GetCapsuleComponent _asbp_super_character)))) (Components|Capsule|GetScaledCapsuleRadius (Variables|/Script/Engine.Character|GetCapsuleComponent _asbp_super_character)) "TraceTypeQuery1" false 0 "None"))
  (return _returnvalue))