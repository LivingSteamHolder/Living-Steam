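; BP_Fences is a fence actor that moves when the charging bull enemy reaches its second phase.
; On BeginPlay it finds and stores the BP_ChargingBull in the level.
; Each Tick during phase 2, it sets its location by constant-speed interpolation from Point1's world position toward Point2's, without sweep.
; The interpolation starts from Point1 rather than the actor's own location.
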(event EventBeginPlay
  (bind _returnvalue (Actor|GetActorOfClass "/Game/Blueprints/EarthTitan/BP_ChargingBull.BP_ChargingBull_C"))
  (Variables|Default|SetChargingEnemy _returnvalue))

(event Collision|EventActorBeginOverlap
  (params (OtherActor :type Actor%20Object%20Reference)))

(event EventTick
  (params (DeltaSeconds :type Float%20%28single-precision%29))
  (if (== (Variables|/Script/LivingSteam.ChargingBull|GetPhaseNumber (Variables|Default|GetChargingEnemy)) 2)
    (Transformation|SetActorLocation (Math|Interpolation|VInterptoConstant (Transformation|GetWorldLocation (Variables|Default|Get%20Point%201)) (Transformation|GetWorldLocation (Variables|Default|GetPoint%202)) DeltaSeconds 4e+02) false false)))

(fn ConstructionScript)