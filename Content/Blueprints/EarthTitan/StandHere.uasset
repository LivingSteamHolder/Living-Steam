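; StandHere is a trigger spot that exposes a linked ShieldSphere while a BP_SuperCharacter stands inside its cylinder hitbox.
; On BeginPlay it hides its own Sphere and applies TotalColor to that sphere's dynamic shield material and the Niagara effect.
; Overlap begin and end toggle the effect's CharacterInside flag, switch ShieldSphere between exposed and protected, and show or hide the Sphere if ShieldSphere is valid.
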(event OnComponentBeginOverlap(HitboxCylinder)
  (params (OverlappedComponent :type Primitive%20Component%20Object%20Reference) (OtherActor :type Actor%20Object%20Reference) (OtherComp :type Primitive%20Component%20Object%20Reference) (OtherBodyIndex :type Integer) (bFromSweep :type Boolean) (SweepResult :type Hit%20Result%20Structure%20%28by%20ref%29))
  (Utilities|Casting|CastToBP_SuperCharacter OtherActor)
  (Development|PrintString "Hello")
  (Class|NiagaraComponent|SetVariableBool (Variables|Default|GetNiagara) "CharacterInside" true)
  (if (Utilities|IsValid (Variables|Default|GetShieldSphere))
    (Default|ExposeSphere (Variables|Default|GetShieldSphere))
    (Rendering|SetVisibility (Variables|Default|GetSphere) true false)))

(event OnComponentEndOverlap(HitboxCylinder)
  (params (OverlappedComponent :type Primitive%20Component%20Object%20Reference) (OtherActor :type Actor%20Object%20Reference) (OtherComp :type Primitive%20Component%20Object%20Reference) (OtherBodyIndex :type Integer))
  (Utilities|Casting|CastToBP_SuperCharacter OtherActor)
  (Class|NiagaraComponent|SetVariableBool (Variables|Default|GetNiagara) "CharacterInside" false)
  (if (Utilities|IsValid (Variables|Default|GetShieldSphere))
    (Default|ProtectSphere (Variables|Default|GetShieldSphere))
    (Rendering|SetVisibility (Variables|Default|GetSphere) false false)))

(event EventBeginPlay
  (Rendering|SetVisibility (Variables|Default|GetSphere) false false)
  (bind _returnvalue (Rendering|Material|CreateDynamicMaterialInstance (Variables|Default|GetSphere) 0 "/Game/VFX/ParticleEffects/Materials/M/MI_ShieldMat_Blue.MI_ShieldMat_Blue" "DynamicShieldMat" :!class /Script/Engine.PrimitiveComponent))
  (Rendering|Material|SetVectorParameterValue _returnvalue "Color" (Variables|Default|GetTotal%20Color) :!class /Script/Engine.MaterialInstanceDynamic)
  (Effects|Components|ParticleSystem|SetColorParameter (Variables|Default|GetNiagara) "Color" (Variables|Default|GetTotal%20Color)))

(event Collision|EventActorBeginOverlap
  (params (OtherActor :type Actor%20Object%20Reference)))

(event EventTick
  (params (DeltaSeconds :type Float%20%28single-precision%29)))

(fn ConstructionScript)