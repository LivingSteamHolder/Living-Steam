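; Spike hazard for the Earth Titan boss that respawns any BP_SuperCharacter overlapping the actor, whether the spikes are raised or not.
; EnableSpikes and RetractSpikes write per-segment target heights for the two cube segments; their in-loop Delay does not stagger the writes.
; Tick feeds each target through FInterpToConstant, reading world Z but setting relative location, and repeats the overlap check per segment.
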(event Custom|RetractSpikes
  (Development|PrintString "retract")
  (for (_ _array_index) (Variables|Default|GetSpikeSegments)
    (Utilities|Array|SetArrayElem (Variables|Default|GetFloat) _array_index 0.0)
    (Utilities|FlowControl|Delay 2.0)))

(event Custom|EnableSpikes
  (Development|PrintString "Enable")
  (for (_ _array_index) (Variables|Default|GetSpikeSegments)
    (Utilities|Array|SetArrayElem (Variables|Default|GetFloat) _array_index 4e+01)
    (Utilities|FlowControl|Delay 2.0)))

(event EventBeginPlay
  (Utilities|Array|Add (Variables|Default|GetSpikeSegments) (Variables|Default|GetCube1))
  (Utilities|Array|Add (Variables|Default|GetSpikeSegments) (Variables|Default|Getcube2)))

(event Collision|EventActorBeginOverlap
  (params (OtherActor :type Actor%20Object%20Reference)))

(event EventTick
  (params (DeltaSeconds :type Float%20%28single-precision%29))
  (bind _overlappingactors (Collision|GetOverlappingActors "/Game/Blueprints/BP_SuperCharacter.BP_SuperCharacter_C" :!class /Script/Engine.Actor))
  (for (_array_element _array_index) (Variables|Default|GetSpikeSegments)
    (Transformation|SetRelativeLocation _array_element (Math|Vector|MakeVector 0.0 0.0 (Math|Interpolation|FInterptoConstant (.z (Transformation|GetWorldLocation _array_element)) (Utilities|Array|Get(acopy) (Variables|Default|GetFloat) _array_index) DeltaSeconds 0.0)) false false)
    (if (Utilities|Array|IsNotEmpty _overlappingactors)
      (for _array_element_2 _overlappingactors
        (bind _asbp_super_character (Utilities|Casting|CastToBP_SuperCharacter _array_element_2))
        (Default|RespawnPlayer _asbp_super_character)))))

(fn ConstructionScript)