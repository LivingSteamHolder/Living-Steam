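; Charging bull enemy for the Earth Titan encounter that respawns the player on overlap and shatters destroyable pillars while charging.
; Pillar impacts break Chaos geometry collections with a radial force field, record the destruction and make the bull vulnerable.
; Tick toggles three pillar shields, overlay, Niagara and force from vulnerability in phase one, otherwise starts phase two on shield spheres and stand-here actors once.
; Charge VFX briefly enables custom depth.
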(event Custom|ChargingVFX
  (Development|PrintString "isCharging")
  (Rendering|SetRenderCustomDepth (Variables|Default|GetBody) true)
  (Utilities|FlowControl|Delay 1.0)
  (CallFunction|StopChargingVFX))

(event Custom|StopChargingVFX
  (Development|PrintString "stoppedCharging")
  (Rendering|SetRenderCustomDepth (Variables|Default|GetBody) false))

(event EventBeginPlay)

(event Collision|EventActorBeginOverlap
  (params (OtherActor :type Actor%20Object%20Reference))
  (bind _asbp_super_character (Utilities|Casting|CastToBP_SuperCharacter OtherActor)
    (:then
      (Class|SuperCharacterClass|Respawn _asbp_super_character))
    (:CastFailed
      (bind _asbp_destroyable_pillar (Utilities|Casting|CastToBP_DestroyablePillar OtherActor))
      (Variables|Default|SetOther _asbp_destroyable_pillar)
      (if (Variables|Default|GetbIsCharging)
        (Variables|/Script/GeometryCollectionEngine.GeometryCollectionComponent|SetbEnableDamageFromCollision (Variables|/Game/Blueprints/EarthTitan/BP_DestroyablePillar.BP_DestroyablePillar_C|GetGeometryCollection (Variables|Default|GetOther)) true)
        (Variables|/Script/GeometryCollectionEngine.GeometryCollectionComponent|SetEnableClustering (Variables|/Game/Blueprints/EarthTitan/BP_DestroyablePillar.BP_DestroyablePillar_C|GetGeometryCollection (Variables|Default|GetOther)) false)
        (Utilities|FlowControl|Delay 0.1)
        (Class|FieldSystemComponent|ApplyPhysicsField (Variables|Default|GetFieldSystem) true "Field_LinearForce" 0 (Field|SetRadialVector (Variables|Default|GetRadialVector) (Variables|Default|GetForce%20Strength) (Transformation|GetWorldLocation (Variables|Default|GetBody))))
        (Collision|SetCollisionResponsetoChannel (Variables|/Game/Blueprints/EarthTitan/BP_DestroyablePillar.BP_DestroyablePillar_C|GetGeometryCollection (Variables|Default|GetOther)) "ECC_GameTraceChannel2" "ECR_Ignore")
        (Collision|SetActorEnableCollision (Variables|Default|GetOther) false)
        (Class|ChargingBull|AddDestroyedPillar)
        (Variables|Default|SetbVulnerable true)
        (Variables|/Game/Blueprints/EarthTitan/BP_DestroyablePillar.BP_DestroyablePillar_C|SetisAlive (Variables|Default|GetOther) false)))))

(event Collision|EventHit
  (params (MyComp :type Primitive%20Component%20Object%20Reference) (Other :type Actor%20Object%20Reference) (OtherComp :type Primitive%20Component%20Object%20Reference) (bSelfMoved :type Boolean) (HitLocation :type Vector :default "0, 0, 0") (HitNormal :type Vector :default "0, 0, 0") (NormalImpulse :type Vector :default "0, 0, 0") (Hit :type Hit%20Result%20Structure%20%28by%20ref%29)))

(event EventTick
  (params (DeltaSeconds :type Float%20%28single-precision%29))
  (bind _pillar_3 (Variables|Default|GetPillar%203))
  (bind _body (Variables|Default|GetBody))
  (bind _niagara (Variables|Default|GetNiagara))
  (bind _pillar_1 (Variables|Default|GetPillar%201))
  (bind _pillar_2 (Variables|Default|GetPillar%202))
  (if (== (Variables|Default|GetPhaseNumber) 1)
    (if (Variables|Default|GetbVulnerable)
      (bind _aspillar_shield_blueprint (Utilities|Casting|CastToPillarShield_Blueprint _pillar_1))
      (Variables|/Game/Blueprints/PillarShield_Blueprint.PillarShield_Blueprint_C|SetDisableShield _aspillar_shield_blueprint false)
      (bind _aspillar_shield_blueprint_2 (Utilities|Casting|CastToPillarShield_Blueprint _pillar_2))
      (Variables|/Game/Blueprints/PillarShield_Blueprint.PillarShield_Blueprint_C|SetDisableShield _aspillar_shield_blueprint_2 false)
      (bind _aspillar_shield_blueprint_3 (Utilities|Casting|CastToPillarShield_Blueprint _pillar_3))
      (Variables|/Game/Blueprints/PillarShield_Blueprint.PillarShield_Blueprint_C|SetDisableShield _aspillar_shield_blueprint_3 false)
      (Rendering|Material|SetOverlayMaterial _body 0 :!class /Script/Engine.MeshComponent)
      (Rendering|SetVisibility _niagara false true)
      (Variables|/Game/VFX/Basic_impact_UpdateCUBE.Basic_impact_UpdateCUBE_C|SetForce%20Strength (Variables|Default|GetNewVar) 0.0)
      (else
        (bind _aspillar_shield_blueprint_4 (Utilities|Casting|CastToPillarShield_Blueprint _pillar_1))
        (Variables|/Game/Blueprints/PillarShield_Blueprint.PillarShield_Blueprint_C|SetDisableShield _aspillar_shield_blueprint_4 true)
        (bind _aspillar_shield_blueprint_5 (Utilities|Casting|CastToPillarShield_Blueprint _pillar_2))
        (Variables|/Game/Blueprints/PillarShield_Blueprint.PillarShield_Blueprint_C|SetDisableShield _aspillar_shield_blueprint_5 true)
        (bind _aspillar_shield_blueprint_6 (Utilities|Casting|CastToPillarShield_Blueprint _pillar_3))
        (Variables|/Game/Blueprints/PillarShield_Blueprint.PillarShield_Blueprint_C|SetDisableShield _aspillar_shield_blueprint_6 true)
        (Rendering|Material|SetOverlayMaterial _body "/Game/VFX/ParticleEffects/Materials/MI/MI_BlueOverlay.MI_BlueOverlay" :!class /Script/Engine.MeshComponent)
        (Rendering|SetVisibility _niagara true true)
        (Variables|/Game/VFX/Basic_impact_UpdateCUBE.Basic_impact_UpdateCUBE_C|SetForce%20Strength (Variables|Default|GetNewVar) 2.5571748e+10)))
    (else
      (bind _asbp_shield_sphere (Utilities|Casting|CastToBP_ShieldSphere (Variables|Default|GetShieldSphere%201)))
      (Utilities|FlowControl|DoOnce false
        (:Completed
          (Default|Phase2Start _asbp_shield_sphere)
          (bind _asbp_shield_sphere_2 (Utilities|Casting|CastToBP_ShieldSphere (Variables|Default|GetShieldSphere%202)))
          (Default|Phase2Start _asbp_shield_sphere_2)
          (Default|Phase2Start (Variables|Default|Getstand%20here%20array) 0.0))))))

(fn ConstructionScript
  (Variables|Default|Setstand%20here%20array (Utilities|Array|MakeArray (Variables|Default|GetStand%20here%201) (Variables|Default|GetStand%20here%202))))