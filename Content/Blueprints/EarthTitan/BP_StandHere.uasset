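; BP_StandHere is an Earth Titan stand-here zone that exposes its linked shield sphere and disables its shields while a BP_SuperCharacter is inside.
; Hitbox overlaps toggle the sphere state, the zone's shield mesh and a Niagara flag.
; The construction script colors zone and linked sphere, dividing by HSV value to drop emissive intensity, and applies ring size presets.
; In the boss version, the zone effect stays off until Phase2Start.
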(event OnComponentBeginOverlap(HitboxCylinder)
  (params (OverlappedComponent :type Primitive%20Component%20Object%20Reference) (OtherActor :type Actor%20Object%20Reference) (OtherComp :type Primitive%20Component%20Object%20Reference) (OtherBodyIndex :type Integer) (bFromSweep :type Boolean) (SweepResult :type Hit%20Result%20Structure%20%28by%20ref%29))
  (Utilities|Casting|CastToBP_SuperCharacter OtherActor)
  (Development|PrintString "CharacterInside")
  (Class|NiagaraComponent|SetVariableBool (Variables|Default|GetNiagara) "CharacterInside" true)
  (if (Utilities|IsValid (Variables|Default|GetShieldSphere))
    (Default|ExposeSphere (Variables|Default|GetShieldSphere))
    (Rendering|SetVisibility (Variables|Default|GetSphere) true false)
    (bind _asbp_shield_sphere (Utilities|Casting|CastToBP_ShieldSphere (Variables|Default|GetShieldSphere)))
    (Default|DisableShields _asbp_shield_sphere)))

(event OnComponentEndOverlap(HitboxCylinder)
  (params (OverlappedComponent :type Primitive%20Component%20Object%20Reference) (OtherActor :type Actor%20Object%20Reference) (OtherComp :type Primitive%20Component%20Object%20Reference) (OtherBodyIndex :type Integer))
  (Utilities|Casting|CastToBP_SuperCharacter OtherActor)
  (Class|NiagaraComponent|SetVariableBool (Variables|Default|GetNiagara) "CharacterInside" false)
  (if (Utilities|IsValid (Variables|Default|GetShieldSphere))
    (Default|ProtectSphere (Variables|Default|GetShieldSphere))
    (Rendering|SetVisibility (Variables|Default|GetSphere) false false)
    (bind _asbp_shield_sphere (Utilities|Casting|CastToBP_ShieldSphere (Variables|Default|GetShieldSphere)))
    (Default|InitiateShields _asbp_shield_sphere)))

(event Custom|Phase2Start
  (params (DeltaSeconds :type Float%20%28single-precision%29))
  (Components|Activation|Activate (Variables|Default|GetNiagara) true))

(event EventBeginPlay
  (if (Variables|Default|GetBossVersion)
    (Components|Activation|Deactivate (Variables|Default|GetNiagara))))

(event Collision|EventActorBeginOverlap
  (params (OtherActor :type Actor%20Object%20Reference)))

(fn ConstructionScript
  (bind _total_color (Variables|Default|GetTotal%20Color))
  (bind _shieldsphere (Variables|Default|GetShieldSphere))
  (bind _total_color_2 (Variables|Default|GetTotal%20Color))
  (bind (_r _g _b _a) (Math|Color|BreakColor _total_color))
  (bind (_r_2 _g_2 _b_2) (Math|Color|BreakColor _total_color_2))
  (bind _v (Math|Color|RGBtoHSV(LinearColor) _total_color_2))
  (bind _returnvalue (Rendering|Material|CreateDynamicMaterialInstance (Variables|Default|GetSphere) 0 "/Game/VFX/ParticleEffects/Materials/M/MI_ShieldMat_Blue.MI_ShieldMat_Blue" "DynamicShieldMat" :!class /Script/Engine.PrimitiveComponent))
  (Rendering|Material|SetVectorParameterValue _returnvalue "Color" (Variables|Default|GetTotal%20Color) :!class /Script/Engine.MaterialInstanceDynamic)
  (Effects|Components|ParticleSystem|SetColorParameter (Variables|Default|GetNiagara) "Color" (Variables|Default|GetTotal%20Color))
  (if (Utilities|IsValid _shieldsphere)
    ;[1 1 1] Matches the color of the sphere to that of the zone
    (bind _asbp_shield_sphere (Utilities|Casting|CastToBP_ShieldSphere _shieldsphere))
    (bind _output_get (Variables|Default|SetSphere%20Color (Utilities|Struct|MakeLinearColor (/ _r_2 _v) (/ _g_2 _v) (/ _b_2 _v) 0.5)))
    (Effects|Components|ParticleSystem|SetColorParameter (Variables|/Game/Blueprints/EarthTitan/BP_ShieldSphere.BP_ShieldSphere_C|GetNiagara _asbp_shield_sphere) "Color" _output_get)
    (bind _asbp_shield_sphere_2 (Utilities|Casting|CastToBP_ShieldSphere (Variables|Default|GetShieldSphere)))
    ;[1 1 1] Sets the color of the rings to match the color of the zone
    (bind _output_get_2 (Variables|Default|SetSphere%20Color (Utilities|Struct|MakeLinearColor _r _g _b _a)))
    (Effects|Components|ParticleSystem|SetColorParameter (Variables|/Game/Blueprints/EarthTitan/BP_ShieldSphere.BP_ShieldSphere_C|GetNiagara1 _asbp_shield_sphere_2) "Color" _output_get_2))
  ;[1 1 1] Size Presets
  ;;[1 1 1] Small Size
  (if (Utilities|Enum|Equal(Enum) (Variables|Default|GetSize%20Preset) "NewEnumerator0")
    (Effects|Components|ParticleSystem|SetFloatParameter (Variables|Default|GetNiagara) "width" 1.0)
    (Effects|Components|ParticleSystem|SetFloatParameter (Variables|Default|GetNiagara) "RingSize" 1e+02)
    (else
      ;;[1 1 1] Medium Size
      (if (Utilities|Enum|Equal(Enum) (Variables|Default|GetSize%20Preset) "NewEnumerator1")
        (Effects|Components|ParticleSystem|SetFloatParameter (Variables|Default|GetNiagara) "width" 2.0)
        (Effects|Components|ParticleSystem|SetFloatParameter (Variables|Default|GetNiagara) "RingSize" 5e+02)
        (else
          ;;[1 1 1] Big Size
          (if (Utilities|Enum|Equal(Enum) (Variables|Default|GetSize%20Preset) "NewEnumerator2")
            (Effects|Components|ParticleSystem|SetFloatParameter (Variables|Default|GetNiagara) "width" 1e+01)
            (Effects|Components|ParticleSystem|SetFloatParameter (Variables|Default|GetNiagara) "RingSize" 2e+03)))))))