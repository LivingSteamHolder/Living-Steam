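; BP_SafePad is an Earth Titan platform actor that caches the player and the BP_ChargingBull boss.
; DestroyPlattform hides its cylinder mesh but is not called within this Blueprint.
; Tick runs a ten-second timer, then calls RespawnPlattform once neither player nor boss overlaps the pad.
; Despite its name, RespawnPlattform also hides the cylinder, disables actor collision and resets the timer, so nothing here restores the pad.
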(event Custom|Destroy%20Plattform
  (Rendering|SetVisibility (Variables|Default|GetCylinder) false false))

(event Custom|Respawn%20Plattform
  (Rendering|SetVisibility (Variables|Default|GetCylinder) false false)
  (Collision|SetActorEnableCollision false)
  (Variables|Default|SetRespawnCooldown 0.0))

(event EventBeginPlay
  (Variables|Default|SetPlayerRef (Game|GetPlayerCharacter 0))
  (bind _returnvalue (Actor|GetActorOfClass "/Game/Blueprints/EarthTitan/BP_ChargingBull.BP_ChargingBull_C"))
  (Variables|Default|SetBossRef _returnvalue))

(event Collision|EventActorBeginOverlap
  (params (OtherActor :type Actor%20Object%20Reference)))

(event EventTick
  (params (DeltaSeconds :type Float%20%28single-precision%29))
  (bind _output_get (Variables|Default|SetRespawnCooldown (+ DeltaSeconds (Variables|Default|GetRespawnCooldown))))
  (if (>= _output_get 1e+01)
    (if (and (!= (Collision|IsOverlappingActor (Variables|Default|GetPlayerRef) :!class /Script/Engine.Actor) true) (!= (Collision|IsOverlappingActor (Variables|Default|GetBossRef) :!class /Script/Engine.Actor) true))
      (CallFunction|RespawnPlattform))))

(fn ConstructionScript)