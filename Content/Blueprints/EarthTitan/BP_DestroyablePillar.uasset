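; Destructible pillar in the Earth Titan content whose collision and look follow the state of the charging bull.
; It finds BP_ChargingBull on BeginPlay, then polls its Vulnerable flag every Tick.
; While the bull is vulnerable, pillar and bull ignore each other's collision channels and the Geometry Collection turns gold.
; Otherwise the pillar overlaps Vehicle, the bull's body blocks Destructible, and the base material returns.
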(event EventBeginPlay
  (bind _returnvalue (Actor|GetActorOfClass "/Game/Blueprints/EarthTitan/BP_ChargingBull.BP_ChargingBull_C"))
  (Variables|Default|SetChargingBull _returnvalue)
  (Variables|Default|SetisDestroyable true))

(event Collision|EventActorBeginOverlap
  (params (OtherActor :type Actor%20Object%20Reference)))

(event EventTick
  (params (DeltaSeconds :type Float%20%28single-precision%29))
  (bind _geometrycollection (Variables|Default|GetGeometryCollection))
  (bind _chargingbull (Variables|Default|GetChargingBull))
  (bind _body (Variables|/Game/Blueprints/EarthTitan/BP_ChargingBull.BP_ChargingBull_C|GetBody _chargingbull))
  (if (Variables|/Script/LivingSteam.ChargingBull|GetbVulnerable _chargingbull)
    (Collision|SetCollisionResponsetoChannel (Variables|Default|GetGeometryCollection) "ECC_Vehicle" "ECR_Ignore")
    (Collision|SetCollisionResponsetoChannel _body "ECC_Destructible" "ECR_Ignore")
    (Rendering|Material|SetMaterial _geometrycollection 0 "/Game/StarterContent/Materials/M_Metal_Gold.M_Metal_Gold")
    (else
      (Collision|SetCollisionResponsetoChannel (Variables|Default|GetGeometryCollection) "ECC_Vehicle" "ECR_Overlap")
      (Collision|SetCollisionResponsetoChannel _body "ECC_Destructible" "ECR_Block")
      (Rendering|Material|SetMaterial _geometrycollection 0 "/Engine/MapTemplates/Materials/BasicAsset01.BasicAsset01"))))

(fn ConstructionScript)