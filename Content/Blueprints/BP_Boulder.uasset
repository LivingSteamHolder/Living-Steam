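; Rolling boulder hazard that travels along a spline, respawning any BP_SuperCharacter its sphere touches.
; StartBoulder enables Tick after an initial delay, and Tick advances the sphere by speed, spinning its roll while taking pitch and yaw from the spline.
; Past the spline's end, a delay precedes resetting the distance to restart the run.
; A separate trigger starts and stops the character's camera shake on overlap, using a flag to avoid restarting it.
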(event OnComponentBeginOverlap(Trigger)
  (params (OverlappedComponent :type Primitive%20Component%20Object%20Reference) (OtherActor :type Actor%20Object%20Reference) (OtherComp :type Primitive%20Component%20Object%20Reference) (OtherBodyIndex :type Integer) (bFromSweep :type Boolean) (SweepResult :type Hit%20Result%20Structure%20%28by%20ref%29))
  (bind _asbp_super_character (Utilities|Casting|CastToBP_SuperCharacter OtherActor))
  (if (not (Variables|/Game/Blueprints/BP_SuperCharacter.BP_SuperCharacter_C|GetIsCameraShakePlaying _asbp_super_character))
    (Variables|/Game/Blueprints/BP_SuperCharacter.BP_SuperCharacter_C|SetIsCameraShakePlaying _asbp_super_character true)
    (CameraShake|Start (Variables|/Game/Blueprints/BP_SuperCharacter.BP_SuperCharacter_C|GetCameraShakeSource _asbp_super_character))))

(event OnComponentEndOverlap(Trigger)
  (params (OverlappedComponent :type Primitive%20Component%20Object%20Reference) (OtherActor :type Actor%20Object%20Reference) (OtherComp :type Primitive%20Component%20Object%20Reference) (OtherBodyIndex :type Integer))
  (bind _asbp_super_character (Utilities|Casting|CastToBP_SuperCharacter OtherActor))
  (CameraShake|StopAllCameraShakes (Variables|/Game/Blueprints/BP_SuperCharacter.BP_SuperCharacter_C|GetCameraShakeSource _asbp_super_character) false)
  (Variables|/Game/Blueprints/BP_SuperCharacter.BP_SuperCharacter_C|SetIsCameraShakePlaying _asbp_super_character false))

(event OnComponentBeginOverlap(Sphere)
  (params (OverlappedComponent :type Primitive%20Component%20Object%20Reference) (OtherActor :type Actor%20Object%20Reference) (OtherComp :type Primitive%20Component%20Object%20Reference) (OtherBodyIndex :type Integer) (bFromSweep :type Boolean) (SweepResult :type Hit%20Result%20Structure%20%28by%20ref%29))
  (bind _asbp_super_character (Utilities|Casting|CastToBP_SuperCharacter OtherActor))
  (Default|RespawnPlayer _asbp_super_character))

(event Custom|StartBoulder
  (Utilities|FlowControl|Delay (Variables|Default|GetTimeBeforeSpawningFirstTime))
  (Actor|Tick|SetActorTickEnabled true))

(event EventTick
  (params (DeltaSeconds :type Float%20%28single-precision%29))
  (bind _sphere (Variables|Default|GetSphere))
  (bind _output_get (Variables|Default|SetDistanceAlongSpline (+ (* DeltaSeconds (Variables|Default|GetSpeed)) (Variables|Default|GetDistanceAlongSpline))))
  (Transformation|AddLocalRotation _sphere (Math|Rotator|MakeRotator (Variables|Default|GetRollSpeed) 0.0 0.0) false false)
  (Transformation|SetRelativeTransform _sphere (Math|Transform|MakeTransform (.location (Spline|GetTransformatDistanceAlongSpline (Variables|Default|GetSpline) _output_get "Local" false)) (Math|Rotator|MakeRotator (.roll (Variables|/Script/Engine.SceneComponent|GetRelativeRotation _sphere)) (.pitch (.rotation (Spline|GetTransformatDistanceAlongSpline (Variables|Default|GetSpline) _output_get "Local" false))) (- (.yaw (.rotation (Spline|GetTransformatDistanceAlongSpline (Variables|Default|GetSpline) _output_get "Local" false))) 9e+01)) (Variables|/Script/Engine.SceneComponent|GetRelativeScale3D _sphere)) false false)
  (if (> (Variables|Default|GetDistanceAlongSpline) (Spline|GetSplineLength (Variables|Default|GetSpline)))
    (Utilities|FlowControl|Delay (Variables|Default|GetDelayBetweenSpawnsInSeconds))
    (Variables|Default|SetDistanceAlongSpline 0.0)))

(fn ConstructionScript)

(fn MoveSphereAlongSpline
  (params (A :type Float%20%28double-precision%29)))