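; BP_BoulderCOPY_LEO is a rolling boulder hazard that follows a spline and respawns any BP_SuperCharacter that overlaps it.
; Each Tick advances the distance by Speed, spins the Sphere on roll, and takes its location, pitch and offset yaw from the spline.
; MSSRollingBoulder copies the Sphere's transform every frame.
; When ShouldLoop is set, the distance resets to zero past the spline's end.
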(event Collision|EventActorBeginOverlap
  (params (OtherActor :type Actor%20Object%20Reference))
  (bind _asbp_super_character (Utilities|Casting|CastToBP_SuperCharacter OtherActor))
  (Default|RespawnPlayer _asbp_super_character))

(event EventTick
  (params (DeltaSeconds :type Float%20%28single-precision%29))
  (bind _sphere (Variables|Default|GetSphere))
  (bind _output_get (Variables|Default|SetDistanceAlongSpline (+ (* DeltaSeconds (Variables|Default|GetSpeed)) (Variables|Default|GetDistanceAlongSpline))))
  (Transformation|AddLocalRotation _sphere (Math|Rotator|MakeRotator (Variables|Default|GetRollSpeed) 0.0 0.0) false false)
  (Transformation|SetRelativeTransform _sphere (Math|Transform|MakeTransform (.location (Spline|GetTransformatDistanceAlongSpline (Variables|Default|GetSpline) _output_get "Local" false)) (Math|Rotator|MakeRotator (.roll (Variables|/Script/Engine.SceneComponent|GetRelativeRotation _sphere)) (.pitch (.rotation (Spline|GetTransformatDistanceAlongSpline (Variables|Default|GetSpline) _output_get "Local" false))) (- (.yaw (.rotation (Spline|GetTransformatDistanceAlongSpline (Variables|Default|GetSpline) _output_get "Local" false))) 9e+01)) (Variables|/Script/Engine.SceneComponent|GetRelativeScale3D _sphere)) false false)
  (Transformation|SetRelativeTransform (Variables|Default|GetMSS_RollingBoulder) (Transformation|GetRelativeTransform (Variables|Default|GetSphere)) false false)
  (if (Variables|Default|GetShouldLoop)
    (if (> (Variables|Default|GetDistanceAlongSpline) (Spline|GetSplineLength (Variables|Default|GetSpline)))
      (Variables|Default|SetDistanceAlongSpline 0.0))))

(fn ConstructionScript)