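; BP_PillarSound drives a pillar shield's MetaSound audio, running as a child actor of PillarShield_Blueprint.
; BeginPlay caches the parent shield, and Tick polls its state, fading the sound out while DisableShield is set.
; When the shield is not disabled and its pillar is alive, a DoOnce, reset during disable, fades the sound in and fires the StartShield trigger parameter, with a debug print.
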(event EventBeginPlay
  (bind _aspillar_shield_blueprint (Utilities|Casting|CastToPillarShield_Blueprint (Actor|GetParentActor)))
  (Variables|Default|SetAs%20Pillar%20Shield%20Blueprint _aspillar_shield_blueprint))

(event Collision|EventActorBeginOverlap
  (params (OtherActor :type Actor%20Object%20Reference)))

(event EventTick
  (params (DeltaSeconds :type Float%20%28single-precision%29))
  (if (Variables|/Game/Blueprints/PillarShield_Blueprint.PillarShield_Blueprint_C|GetDisableShield (Variables|Default|GetAs%20Pillar%20Shield%20Blueprint))
    (Audio|Components|Audio|FadeOut (Variables|Default|GetMSS_PillarSounds) 0.2 0.0 "Linear" :!class /Script/Engine.AudioComponent)
    (goto _label Reset)
    (elif (Variables|/Game/Blueprints/EarthTitan/BP_DestroyablePillar.BP_DestroyablePillar_C|GetisAlive (Variables|/Game/Blueprints/PillarShield_Blueprint.PillarShield_Blueprint_C|GetPillar (Variables|Default|GetAs%20Pillar%20Shield%20Blueprint)))
      (Utilities|FlowControl|DoOnce false :!label _label
        (:Completed
          (Audio|Components|Audio|FadeIn (Variables|Default|GetMSS_PillarSounds) 0.2 1.0 0.0 "Linear" :!class /Script/Engine.AudioComponent)
          (Class|AudioParameterControllerInterface|SetTriggerParameter (Variables|Default|GetMSS_PillarSounds) "StartShield")
          (Development|PrintString "Fade"))))))

(fn ConstructionScript)