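; BP_BullSounds is a sound helper actor that plays spatialized audio for its parent BP_ChargingBull.
; It caches the parent on BeginPlay, then polls its charging, rotating and preparing-to-charge flags every Tick.
; DoOnce gates turn those flags into one-shot cues at the bull's location: a layered attack with a delayed repeat, a rotate sound, and a charge-up.
; Each new rotation re-arms the charge-up gate.
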(event EventBeginPlay
  (bind _asbp_charging_bull (Utilities|Casting|CastToBP_ChargingBull (Actor|GetParentActor)))
  (Variables|Default|SetAs%20BP%20Charging%20Bull _asbp_charging_bull))

(event Collision|EventActorBeginOverlap
  (params (OtherActor :type Actor%20Object%20Reference)))

(event EventTick
  (params (DeltaSeconds :type Float%20%28single-precision%29))
  (bind _as_bp_charging_bull (Variables|Default|GetAs%20BP%20Charging%20Bull))
  (bind _as_bp_charging_bull_2 (Variables|Default|GetAs%20BP%20Charging%20Bull))
  (bind _as_bp_charging_bull_3 (Variables|Default|GetAs%20BP%20Charging%20Bull))
  (bind _returnvalue (Transformation|GetActorLocation _as_bp_charging_bull_2))
  (Utilities|FlowControl|Sequence
    (:then_0
      (if (Variables|/Script/LivingSteam.ChargingBull|GetbIsCharging _as_bp_charging_bull_2)
        (Utilities|FlowControl|DoOnce false :!label _label
          (:Completed
            (Audio|PlaySoundatLocation "/Game/Sounds/Waves/Enemy/SW_BullAttack1.SW_BullAttack1" _returnvalue "0, 0, 0" 1.0 5.0 0.0 "/Game/Sounds/SA_Bull.SA_Bull" 0 0 0)
            (Audio|PlaySoundatLocation "/Game/Sounds/Waves/Enemy/Underwater_Swoosh2.Underwater_Swoosh2" _returnvalue "0, 0, 0" 2.0 1.0 0.0 "/Game/Sounds/SA_Bull.SA_Bull" 0 0 0)
            (Audio|PlaySoundatLocation "/Game/Sounds/Waves/Enemy/RockMonster_HurtGrowl8.RockMonster_HurtGrowl8" _returnvalue "0, 0, 0" 2.0 1.0 0.0 "/Game/Sounds/SA_Bull.SA_Bull" 0 0 0)
            (Utilities|FlowControl|Delay 0.7)
            (Audio|PlaySoundatLocation "/Game/Sounds/Waves/Enemy/SW_BullAttack1.SW_BullAttack1" _returnvalue "0, 0, 0" 1.0 5.0 0.0 "/Game/Sounds/SA_Bull.SA_Bull" 0 0 0)))
        (else
          (goto _label Reset))))
    (:then_1
      (if (Variables|/Script/LivingSteam.ChargingBull|GetIsRotating _as_bp_charging_bull_3)
        (Utilities|FlowControl|DoOnce false :!label _label_2
          (:Completed
            (Audio|PlaySoundatLocation "/Game/Sounds/Waves/Enemy/Rotate/SW_Rotate1.SW_Rotate1" (Transformation|GetActorLocation _as_bp_charging_bull_3) "0, 0, 0" 1.0 2.0 0.0 "/Game/Sounds/SA_Bull.SA_Bull" 0 0 0)
            (goto _label_3 Reset)))
        (else
          (goto _label_2 Reset))))
    (:then_2
      (if (Variables|/Script/LivingSteam.ChargingBull|GetIsPreparingToCharge _as_bp_charging_bull)
        (Utilities|FlowControl|DoOnce false :!label _label_3
          (:Completed
            (Audio|PlaySoundatLocation "/Game/Sounds/Waves/Enemy/ChargeUp/SW_Chargeup1.SW_Chargeup1" (Transformation|GetActorLocation _as_bp_charging_bull) "0, 0, 0" 1.0 5.0 0.0 "/Game/Sounds/SA_Bull.SA_Bull" 0 0 0)))))))

(fn ConstructionScript)