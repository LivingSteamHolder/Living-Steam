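; PillarShield is an actor Blueprint for a shield whose visible mesh is tied to a referenced Pillar.
; Every Tick it shows the static mesh only while the Pillar is alive and DisableShield is false, and hides it otherwise.
; It polls this state each frame and changes only visibility, with no collision or damage logic in its graphs.
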(event EventBeginPlay)

(event Collision|EventActorBeginOverlap
  (params (OtherActor :type Actor%20Object%20Reference)))

(event EventTick
  (params (DeltaSeconds :type Float%20%28single-precision%29))
  (if (Variables|/Game/Blueprints/EarthTitan/BP_DestroyablePillar.BP_DestroyablePillar_C|GetisAlive (Variables|Default|GetPillar))
    (if (Variables|Default|GetDisableShield)
      (Rendering|SetVisibility (Variables|Debug|GetStaticMeshComponent) false false)
      (else
        (Rendering|SetVisibility (Variables|Debug|GetStaticMeshComponent) true false)))
    (else
      (Rendering|SetVisibility (Variables|Debug|GetStaticMeshComponent) false false))))

(fn ConstructionScript)