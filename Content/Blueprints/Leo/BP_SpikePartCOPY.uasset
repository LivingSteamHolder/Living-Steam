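; Moving spike hazard that respawns a BP_SuperCharacter overlapping its mesh.
; Tick moves the actor toward Target at constant speed, firing the SpikeRise sound trigger once each time it rises above a height threshold.
; AudioComp yaws smoothly toward the player with an offset, and spike sounds drop attenuation and spatialization while IsPlayerOnTop is set.
; BeginPlay positions the sound from the mesh bounds and copies that mesh to SoundDetection.
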(event OnComponentBeginOverlap(StaticMesh)
  (params (OverlappedComponent :type Primitive%20Component%20Object%20Reference) (OtherActor :type Actor%20Object%20Reference) (OtherComp :type Primitive%20Component%20Object%20Reference) (OtherBodyIndex :type Integer) (bFromSweep :type Boolean) (SweepResult :type Hit%20Result%20Structure%20%28by%20ref%29))
  (bind _asbp_super_character (Utilities|Casting|CastToBP_SuperCharacter OtherActor))
  (Default|RespawnPlayer _asbp_super_character))

(event EventBeginPlay
  (bind _staticmesh (Variables|Default|GetStaticMesh))
  (bind _staticmesh_2 (Variables|/Script/Engine.StaticMeshComponent|GetStaticMesh _staticmesh))
  (bind _returnvalue (StaticMesh|GetBoundingBox _staticmesh_2))
  (bind (_x _y) (Math|Vector|BreakVector (.max _returnvalue)))
  (Transformation|SetRelativeLocation (Variables|Default|GetMSS_SpikeSounds) (Math|Vector|MakeVector _x _y 2.5e+02) false false)
  (Components|StaticMesh|SetStaticMesh (Variables|Default|GetSoundDetection) (Variables|/Script/Engine.StaticMeshComponent|GetStaticMesh (Variables|Default|GetStaticMesh))))

(event Collision|EventActorBeginOverlap
  (params (OtherActor :type Actor%20Object%20Reference)))

(event EventTick
  (params (DeltaSeconds :type Float%20%28single-precision%29))
  (bind _returnvalue (Game|GetPlayerCharacter 0))
  (bind _mss_spikesounds (Variables|Default|GetMSS_SpikeSounds))
  (bind _audiocomp (Variables|Default|GetAudioComp))
  (bind _mss_spikesounds_2 (Variables|Default|GetMSS_SpikeSounds))
  (bind _returnvalue_2 (Transformation|GetActorLocation _returnvalue))
  (bind _returnvalue_3 (Transformation|GetWorldLocation _audiocomp))
  (bind _returnvalue_4 (Math|Rotator|FindLookatRotation _returnvalue_3 _returnvalue_2))
  (Transformation|SetWorldRotation (Variables|Default|GetAudioComp) (Math|Rotator|MakeRotator 0.0 0.0 (.yaw (Math|Interpolation|RInterpTo (Transformation|GetWorldRotation _audiocomp) (Math|Rotator|MakeRotator (.roll _returnvalue_4) (.pitch _returnvalue_4) (- (.yaw _returnvalue_4) 45.0)) (Utilities|Time|GetWorldDeltaSeconds) 2e+01))) false false)
  (Utilities|FlowControl|Sequence
    (:then_0
      (Transformation|SetActorLocation (Math|Interpolation|VInterptoConstant (Transformation|GetActorLocation) (Variables|Default|GetTarget) DeltaSeconds 2e+02) false false))
    (:then_1
      (if (>= (.z (Transformation|GetActorLocation)) -7e+02)
        (Utilities|FlowControl|DoOnce false :!label _label
          (:Completed
            (Class|AudioParameterControllerInterface|SetTriggerParameter (Variables|Default|GetMSS_SpikeSounds) "SpikeRise")))
        (else
          (goto _label Reset))))
    (:then_2
      (if (Variables|Default|GetIsPlayerOnTop)
        (Variables|/Script/Engine.AudioComponent|SetAttenuationSettings _mss_spikesounds 0)
        (Variables|/Script/Engine.AudioComponent|SetbOverrideAttenuation _mss_spikesounds true)
        (Variables|/Script/Engine.AudioComponent|SetbAllowSpatialization _mss_spikesounds false)
        (else
          (Variables|/Script/Engine.AudioComponent|SetAttenuationSettings (Variables|Default|GetMSS_SpikeSounds) "/Game/Sounds/Attenuations/SA_Spikes.SA_Spikes")
          (Variables|/Script/Engine.AudioComponent|SetbOverrideAttenuation _mss_spikesounds_2 false)
          (Variables|/Script/Engine.AudioComponent|SetbAllowSpatialization _mss_spikesounds_2 true))))))

(fn ConstructionScript)