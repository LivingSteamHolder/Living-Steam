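; Charging bull enemy pawn, apparently a working copy, that respawns any BP_SuperCharacter it overlaps and moves through a fast FloatingPawnMovement.
; Tick plays a layered attack sound once per charge, re-armed when IsCharging clears; the charge flag is not set in this graph.
; Pillar-breaking via Geometry Collection and a radial physics field is left disconnected, so pillar hits do nothing, and a looping two-second timer drives nothing.
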(event EventBeginPlay
  (Variables|/Script/Engine.FloatingPawnMovement|SetMaxSpeed (Variables|Default|GetFloatingPawnMovement) 4e+03))

(event Collision|EventActorBeginOverlap
  (params (OtherActor :type Actor%20Object%20Reference))
  (bind _asbp_super_character (Utilities|Casting|CastToBP_SuperCharacter OtherActor))
  (Default|RespawnPlayer _asbp_super_character))

(event EventTick
  (params (DeltaSeconds :type Float%20%28single-precision%29))
  (bind _returnvalue (Transformation|GetActorLocation))
  (Utilities|FlowControl|Sequence
    (:then_0
      (Variables|Default|SetTimer (+ (Variables|Default|GetTimer) DeltaSeconds))
      (if (>= (Variables|Default|GetTimer) 2.0)
        (Variables|Default|SetTimer 0.0)))
    (:then_1
      (if (Variables|Default|GetbIsCharging)
        (Utilities|FlowControl|DoOnce false :!label _label
          (:Completed
            (Audio|PlaySoundatLocation "/Game/Sounds/Waves/Enemy/SW_BullAttack1.SW_BullAttack1" _returnvalue "0, 0, 0" 1.0 5.0 0.0 "/Game/Sounds/Attenuations/SA_Bull.SA_Bull" 0 0 0)
            (Audio|PlaySoundatLocation "/Game/Sounds/Waves/Enemy/Underwater_Swoosh2.Underwater_Swoosh2" _returnvalue "0, 0, 0" 1.0 1.0 0.0 "/Game/Sounds/Attenuations/SA_Bull.SA_Bull" 0 0 0)
            (Audio|PlaySoundatLocation "/Game/Sounds/Waves/Enemy/Grunts/RockMonster_HurtGrowl8.RockMonster_HurtGrowl8" _returnvalue "0, 0, 0" 1.0 1.0 0.0 "/Game/Sounds/Attenuations/SA_Bull.SA_Bull" 0 0 0)))
        (else
          (goto _label Reset))))))

(event Collision|EventHit
  (params (MyComp :type Primitive%20Component%20Object%20Reference) (Other :type Actor%20Object%20Reference) (OtherComp :type Primitive%20Component%20Object%20Reference) (bSelfMoved :type Boolean) (HitLocation :type Vector :default "0, 0, 0") (HitNormal :type Vector :default "0, 0, 0") (NormalImpulse :type Vector :default "0, 0, 0") (Hit :type Hit%20Result%20Structure%20%28by%20ref%29))
  (bind _asbp_destroyable_pillar (Utilities|Casting|CastToBP_DestroyablePillar Other))
  (if (Variables|Default|GetbIsCharging)
    _))

(fn ConstructionScript)