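; BP_StandardProjectileCOPY is a projectile Blueprint that gives audio feedback based on what it hits.
; On Hit, it casts the other actor to BP_ChargingBull or BP_ShieldSphere and reads its Vulnerable flag.
; It spawns MSS_ShotHit at the impact, firing a damage, shield or other trigger parameter to match.
; Each outcome also prints a debug string; the graph itself applies no damage.
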(event EventBeginPlay)

(event Collision|EventActorBeginOverlap
  (params (OtherActor :type Actor%20Object%20Reference)))

(event EventTick
  (params (DeltaSeconds :type Float%20%28single-precision%29)))

(event Collision|EventHit
  (params (MyComp :type Primitive%20Component%20Object%20Reference) (Other :type Actor%20Object%20Reference) (OtherComp :type Primitive%20Component%20Object%20Reference) (bSelfMoved :type Boolean) (HitLocation :type Vector :default "0, 0, 0") (HitNormal :type Vector :default "0, 0, 0") (NormalImpulse :type Vector :default "0, 0, 0") (Hit :type Hit%20Result%20Structure%20%28by%20ref%29))
  (bind _asbp_charging_bull (Utilities|Casting|CastToBP_ChargingBull Other)
    (:then
      (if (Variables|/Script/LivingSteam.ChargingBull|GetbVulnerable _asbp_charging_bull)
        (bind _returnvalue (Audio|SpawnSoundatLocation "/Game/Sounds/MetaSounds/MSS_ShotHit.MSS_ShotHit" HitLocation "0, 0, 0" 1.0 1.0 0.0 0 0 :!label _label))
        (Class|AudioParameterControllerInterface|SetTriggerParameter _returnvalue "DamageHit")
        (Development|PrintString "damage")
        (else
          (bind _returnvalue_2 (Audio|SpawnSoundatLocation "/Game/Sounds/MetaSounds/MSS_ShotHit.MSS_ShotHit" HitLocation "0, 0, 0" 1.0 1.0 0.0 0 0 :!label _label_2))
          (Class|AudioParameterControllerInterface|SetTriggerParameter _returnvalue_2 "ShieldHit")
          (Development|PrintString "shield"))))
    (:CastFailed
      (bind _asbp_shield_sphere (Utilities|Casting|CastToBP_ShieldSphere Other)
        (:then
          (if (Variables|/Script/LivingSteam.ShieldSphere|GetbVulnerable _asbp_shield_sphere)
            (goto _label)
            (else
              (goto _label_2))))
        (:CastFailed
          (bind _returnvalue_3 (Audio|SpawnSoundatLocation "/Game/Sounds/MetaSounds/MSS_ShotHit.MSS_ShotHit" HitLocation "0, 0, 0" 1.0 1.0 0.0 0 0))
          (Class|AudioParameterControllerInterface|SetTriggerParameter _returnvalue_3 "OtherHit")
          (Development|PrintString "other"))))))

(fn ConstructionScript)