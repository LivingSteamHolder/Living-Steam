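; BP_SoundTrigger is a one-shot trigger that plays a 2D sound when a BP_SuperCharacter first overlaps it.
; It finds BP_PlayerSounds, fades out its current ambient sound, and fades and pauses the general ambient loop.
; The spawned sound becomes the new current ambient sound at the configured volume.
; When that sound finishes, the general ambience unpauses and fades back up.
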(event Custom|OnAudioFinished_Event
  (Audio|Components|Audio|AdjustVolume (Variables|/Game/Blueprints/BP_PlayerSounds.BP_PlayerSounds_C|GetGenerallAmbientSound (stale Collision|EventActorBeginOverlap _returnvalue)) 0.2 0.8 "Linear" :!class /Script/Engine.AudioComponent)
  (Class|AudioComponent|SetPaused (Variables|/Game/Blueprints/BP_PlayerSounds.BP_PlayerSounds_C|GetGenerallAmbientSound (stale Collision|EventActorBeginOverlap _returnvalue)) false))

(event EventBeginPlay)

(event EventTick
  (params (DeltaSeconds :type Float%20%28single-precision%29)))

(event Collision|EventActorBeginOverlap
  (params (OtherActor :type Actor%20Object%20Reference))
  (Utilities|Casting|CastToBP_SuperCharacter OtherActor)
  (Utilities|FlowControl|DoOnce false
    (:Completed
      (bind _returnvalue (Actor|GetActorOfClass "/Game/Blueprints/BP_PlayerSounds.BP_PlayerSounds_C"))
      (Audio|Components|Audio|FadeOut (Variables|/Game/Blueprints/BP_PlayerSounds.BP_PlayerSounds_C|GetCurrentAmbientSound _returnvalue) 0.2 0.0 "Linear" :!class /Script/Engine.AudioComponent)
      (Audio|Components|Audio|AdjustVolume (Variables|/Game/Blueprints/BP_PlayerSounds.BP_PlayerSounds_C|GetGenerallAmbientSound _returnvalue) 0.3 0.0 "Linear" :!class /Script/Engine.AudioComponent)
      (Utilities|FlowControl|Delay 0.3)
      (Class|AudioComponent|SetPaused (Variables|/Game/Blueprints/BP_PlayerSounds.BP_PlayerSounds_C|GetGenerallAmbientSound _returnvalue) true)
      (bind _returnvalue_2 (Audio|SpawnSound2D (Variables|Default|GetSound) 3.0 1.0 0.0 0 false false))
      (bind _output_get (Variables|/Game/Blueprints/BP_PlayerSounds.BP_PlayerSounds_C|SetCurrentAmbientSound _returnvalue _returnvalue_2))
      (Audio|Components|Audio|SetVolumeMultiplier _output_get (Variables|Default|GetVolume) :!class /Script/Engine.AudioComponent)
      (EventDispatchers|AssignOnAudioFinished _output_get (delegate Custom|OnAudioFinished_Event)))))

(fn ConstructionScript)