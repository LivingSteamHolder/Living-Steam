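; Shield sphere actor with Niagara shield effects and MetaSound audio; its boss version stays hidden until phase 2.
; Phase2Start reveals it, spawns the sound and staggers effect activation.
; Shield events toggle effects and fire sound triggers, while Expose and Protect events swap the material and Vulnerable flag.
; Tick polls SphereHealth and fires a one-time Death sound trigger at zero; nothing here applies damage.
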(event Custom|ExposeSphere
  (Variables|Default|SetbVulnerable true)
  (Rendering|Material|SetMaterial (Variables|Default|GetSphere) 0 "/DatasmithContent/Materials/AliasReference.AliasReference"))

(event Custom|ProtectSphere
  (Variables|Default|SetbVulnerable false)
  (Rendering|Material|SetMaterial (Variables|Default|GetSphere) 0 "/Engine/BasicShapes/BasicShapeMaterial.BasicShapeMaterial"))

(event Custom|Disable%20Shields
  (Class|AudioParameterControllerInterface|SetTriggerParameter (Variables|Default|GetMSS) "NoShield")
  (Components|Activation|Deactivate (Variables|Default|GetNiagara))
  (for _array_element (Variables|Default|GetShield%20Effects)
    (Components|Activation|Deactivate _array_element)
    (Development|PrintString "Shields Disabled")
    (Components|Activation|Activate (Variables|Default|GetNiagara4) true)))

(event Custom|Phase2Start
  (if (Variables|Default|GetBossVersion)
    (Utilities|FlowControl|Delay 0.1)
    (Rendering|SetVisibility (Variables|Default|GetDefaultSceneRoot) true true)
    (bind _returnvalue (Audio|SpawnSoundatLocation "/Game/Sounds/MetaSounds/MSS_ShieldSphere.MSS_ShieldSphere" (Transformation|GetActorLocation) "0, 0, 0" 1.0 1.0 0.0 0 0))
    (Variables|Default|SetMSS _returnvalue)
    (Components|Activation|Activate (Variables|Default|GetNiagara) true)
    (Utilities|FlowControl|Delay 0.3)
    (Components|Activation|Activate (Variables|Default|GetNiagara1) true)
    (Components|Activation|Activate (Variables|Default|GetNiagara2) true)
    (Components|Activation|Activate (Variables|Default|GetNiagara3) true)
    (Components|Activation|Activate (Variables|Default|GetNiagara4) true)
    (Development|PrintString "Phase 2 Started")))

(event Custom|Initiate%20Shields
  (Class|AudioParameterControllerInterface|SetTriggerParameter (Variables|Default|GetMSS) "ShieldOn")
  (Components|Activation|Activate (Variables|Default|GetNiagara) true)
  (Utilities|FlowControl|Delay 0.3)
  (for _array_element (Variables|Default|GetShield%20Effects)
    (Components|Activation|Activate _array_element true)
    (Development|PrintString "Shields Enabled")))

(event EventBeginPlay
  (if (Variables|Default|GetBossVersion)
    (Rendering|SetVisibility (Variables|Default|GetDefaultSceneRoot) false true)
    (Variables|Default|SetShield%20Effects (Utilities|Array|MakeArray (Variables|Default|GetNiagara1) (Variables|Default|GetNiagara2) (Variables|Default|GetNiagara3)))
    (Rendering|SetVisibility (Variables|Default|GetSphere) false false)))

(event Collision|EventActorBeginOverlap
  (params (OtherActor :type Actor%20Object%20Reference)))

(event EventTick
  (params (DeltaSeconds :type Float%20%28single-precision%29))
  (if (<= (Variables|Default|GetSphereHealth) 0.0)
    (Utilities|FlowControl|DoOnce false
      (:Completed
        (Class|AudioParameterControllerInterface|SetTriggerParameter (Variables|Default|GetMSS) "Death")))))

(fn ConstructionScript)