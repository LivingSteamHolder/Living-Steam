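; BP_WorldHint is a world-placed hint that shows a text widget while something overlaps its trigger sphere.
; BeginPlay hides the Widget component and passes TextContent into its WB_WorldHint user widget.
; Sphere begin and end overlap toggle the widget's visibility, without filtering which actor overlaps.
; The construction script sizes the sphere from the Radius variable, scaled up by a thousand.
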(event OnComponentBeginOverlap(Sphere)
  (params (OverlappedComponent :type Primitive%20Component%20Object%20Reference) (OtherActor :type Actor%20Object%20Reference) (OtherComp :type Primitive%20Component%20Object%20Reference) (OtherBodyIndex :type Integer) (bFromSweep :type Boolean) (SweepResult :type Hit%20Result%20Structure%20%28by%20ref%29))
  (Rendering|SetVisibility (Variables|Default|GetWidget) true true))

(event OnComponentEndOverlap(Sphere)
  (params (OverlappedComponent :type Primitive%20Component%20Object%20Reference) (OtherActor :type Actor%20Object%20Reference) (OtherComp :type Primitive%20Component%20Object%20Reference) (OtherBodyIndex :type Integer))
  (Rendering|SetVisibility (Variables|Default|GetWidget) false true))

(event EventBeginPlay
  (Rendering|SetVisibility (Variables|Default|GetWidget) false true)
  (bind _aswb_world_hint (Utilities|Casting|CastToWB_WorldHint (UserInterface|GetWidget (Variables|Default|GetWidget))))
  (Variables|/Game/Shahin/WB_WorldHint.WB_WorldHint_C|SetContent _aswb_world_hint (Variables|Default|GetTextContent)))

(fn ConstructionScript
  (Components|Sphere|SetSphereRadius (Variables|Default|GetSphere) (* (Variables|Default|GetRadius) 1e+03) true))