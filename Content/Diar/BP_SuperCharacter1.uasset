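; BP_SuperCharacter1 is a character Blueprint that fires a one-time Niagara ranged-attack effect on shoot input and respawns by reloading the current level.
; IA_Shoot spawns RangedAttack1test at FxSpawnerLocation through a DoOnce with no visible reset, with color enabled.
; After a delay, if the Condition flag set by shoot input is true, the effect switches from color to vortex force.
; RespawnPlayer reopens the level by name.
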(event Custom|RespawnPlayer
  (bind _returnvalue (Game|GetCurrentLevelName true))
  (Game|OpenLevel(byName) (Utilities|String|StringToName _returnvalue)))

(event Input|EnhancedActionEvents|EnhancedInputActionIA_Shoot
  (params (ActionValue :type Boolean) (ElapsedSeconds :type Float%20%28double-precision%29) (TriggeredSeconds :type Float%20%28double-precision%29) (InputAction :type Input%20Action%20Object%20Reference :default "/Game/Blueprints/PlayerController/IA_Shoot.IA_Shoot"))
  (:Ongoing
    (if true
      (Utilities|FlowControl|DoOnce false
        (:Completed
          (bind _returnvalue (Niagara|SpawnSystematLocation "/Game/VFX/ParticleEffects/Shoot/RangedAttack1test.RangedAttack1test" (Transformation|GetWorldLocation (Variables|Default|GetFxSpawnerLocation)) "-90.000000,0.000000,0.000000"))
          (Niagara|SetNiagaraVariable(Bool) _returnvalue "Bool_Color" true)
          (Utilities|FlowControl|Delay 2.0)
          (if (stale _output_get)
            (Class|NiagaraComponent|SetVariableBool _returnvalue "Bool_Color" false)
            (Class|NiagaraComponent|SetVariableBool _returnvalue "Bool_VortexForce" true)))))))

(event Input|EnhancedActionEvents|EnhancedInputActionIA_Shoot
  (params (ActionValue :type Boolean) (ElapsedSeconds :type Float%20%28double-precision%29) (TriggeredSeconds :type Float%20%28double-precision%29) (InputAction :type Input%20Action%20Object%20Reference :default "/Game/Blueprints/PlayerController/IA_Shoot.IA_Shoot"))
  (:Ongoing
    (bind _output_get (Variables|Default|SetCondition true))))

(event EventBeginPlay)

(event Collision|EventActorBeginOverlap
  (params (OtherActor :type Actor%20Object%20Reference)))

(fn ConstructionScript)