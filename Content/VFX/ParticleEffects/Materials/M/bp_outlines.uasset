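; Test Blueprint actor that toggles a post-process outline on its Cube mesh through custom depth and stencil.
; ActivateOutlines enables custom depth rendering and writes the Value variable as the stencil value, while DeactivateOutlines turns custom depth off.
; The construction script calls one or the other based on the TestMode flag, so the effect previews in the editor.
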(event Custom|Activate%20Outlines
  (bind _cube (Variables|Default|GetCube))
  (Rendering|SetRenderCustomDepth _cube true)
  (Rendering|SetCustomDepthStencilValue _cube (Variables|Default|GetValue)))

(event Custom|Deactivate%20Outlines
  (Rendering|SetRenderCustomDepth (Variables|Default|GetCube) false))

(event EventBeginPlay)

(event Collision|EventActorBeginOverlap
  (params (OtherActor :type Actor%20Object%20Reference)))

(event EventTick
  (params (DeltaSeconds :type Float%20%28single-precision%29)))

(fn ConstructionScript
  (if (Variables|Default|GetTestMode)
    (CallFunction|ActivateOutlines)
    (else
      (CallFunction|DeactivateOutlines))))